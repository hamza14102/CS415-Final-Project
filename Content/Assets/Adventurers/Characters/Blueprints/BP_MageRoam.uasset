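; BP_MageRoam is a mage enemy that chases the first-person player character and damages it on contact.
; It loops a walking animation directly on the mesh from BeginPlay, and when PawnSensing sees the player it moves toward them with AI Move To.
; A capsule overlap with the player applies damage and then destroys the mage, so each one hits only once.
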(event OnSeePawn(PawnSensing)
  (params (Pawn :type Pawn%20Object%20Reference))
  (bind _asbp_first_person_character (Utilities|Casting|CastToBP_FirstPersonCharacter Pawn))
  (AI|AIMoveTo self "0, 0, 0" _asbp_first_person_character 5.0 false))

(event OnComponentBeginOverlap(Capsule)
  (params (OverlappedComponent :type Primitive%20Component%20Object%20Reference) (OtherActor :type Actor%20Object%20Reference) (OtherComp :type Primitive%20Component%20Object%20Reference) (OtherBodyIndex :type Integer) (bFromSweep :type Boolean) (SweepResult :type Hit%20Result%20Structure%20%28by%20ref%29))
  (bind _self self)
  (bind _asbp_first_person_character (Utilities|Casting|CastToBP_FirstPersonCharacter OtherActor))
  (Game|Damage|ApplyDamage _asbp_first_person_character 1e+01 0 _self)
  (Actor|DestroyActor _self))

(event EventBeginPlay
  (Components|Animation|PlayAnimation (Variables|Character|GetMesh) "/Game/Assets/Adventurers/Characters/Mage/Mage_Anim_Walking_A.Mage_Anim_Walking_A" true))

(fn ConstructionScript)