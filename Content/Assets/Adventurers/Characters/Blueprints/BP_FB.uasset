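; BP_FB is an AI adventurer pawn that roams randomly and shoots arrows when it sees the first-person player.
; AIMoveTo chains random reachable destinations until PawnSensing triggers a chase.
; Sighting also plays a shooting animation on the player's mesh, spawns a delayed arrow and briefly disables movement, while a retriggerable delay clears the sight flag and resumes roaming.
; Tick updates a camera-facing health bar widget.
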(event OnSeePawn(PawnSensing)
  (params (Pawn :type Pawn%20Object%20Reference))
  (bind _arrow1 (Variables|Default|GetArrow1))
  (bind _returnvalue (Transformation|GetWorldTransform _arrow1))
  (bind _asbp_first_person_character (Utilities|Casting|CastToBP_FirstPersonCharacter Pawn))
  (Utilities|FlowControl|Sequence
    (:then_0
      (Variables|Default|SetCanSeeEnemy true)
      (AI|AIMoveTo self (- (Transformation|GetActorLocation _asbp_first_person_character) "") 0 5.0 false
        (:then
          (Components|Animation|PlayAnimation (Variables|/Script/Engine.Character|GetMesh _asbp_first_person_character) "/Game/Assets/Adventurers/Characters/Rogue/Rogue_Anim_1H_Ranged_Shooting.Rogue_Anim_1H_Ranged_Shooting" false :!label _label)
          (Utilities|FlowControl|Delay 1.5)
          (Game|SpawnActorfromClass "/Game/FinalLevel/FinalBoss/ArrowSpawn.ArrowSpawn_C" (Math|Transform|MakeTransform (.location _returnvalue) (Math|Rotator|MakeRotator 0.0 0.0 (+ (.yaw (.rotation _returnvalue)) 2.7e+02)) (.scale _returnvalue)) "Undefined" 0 0)
          (Pawn|Components|CharacterMovement|DisableMovement (Variables|Character|GetCharacterMovement))
          (Utilities|FlowControl|Delay 2.0)
          (Pawn|Components|CharacterMovement|SetMovementMode (Variables|Character|GetCharacterMovement) "MOVE_Walking" 0)
          (CallFunction|RandomRoam))))
    (:then_1
      (Utilities|FlowControl|RetriggerableDelay 0.6)
      (Variables|Default|SetCanSeeEnemy false)
      (CallFunction|RandomRoam))
    (:then_2
      (goto _label))))

(event Custom|Random%20Roam
  (Components|Animation|PlayAnimation (Variables|Character|GetMesh) "/Game/Assets/Adventurers/Characters/Rogue/Rogue_Anim_Running_A.Rogue_Anim_Running_A" true)
  (AI|AIMoveTo self (.RandomLocation (AI|Navigation|GetRandomReachablePointinRadius (Transformation|GetActorLocation) 2e+03 0 0)) 0 5.0 false
    (:OnSuccess
      (CallFunction|RandomRoam))))

(event EventBeginPlay
  (Utilities|FlowControl|Sequence
    (:then_0
      (Components|Animation|PlayAnimation (Variables|Character|GetMesh) "/Game/Assets/Adventurers/Characters/Barbarian/Barbarian_Anim_Walking_B.Barbarian_Anim_Walking_B" true))
    (:then_1
      (CallFunction|RandomRoam))))

(event Collision|EventActorBeginOverlap
  (params (OtherActor :type Actor%20Object%20Reference)))

(event EventTick
  (params (DeltaSeconds :type Float%20%28single-precision%29))
  (bind _health_bar_widget (Variables|Default|GetHealth%20Bar%20Widget))
  (bind _asbp_fbhealth (Utilities|Casting|CastToBP_FBHealth (UserInterface|GetWidget (Variables|Default|GetHealth%20Bar%20Widget))))
  (Progress|SetPercent (Variables|/Game/Assets/Adventurers/Characters/Blueprints/BP_FBHealth.BP_FBHealth_C|GetHealthBar _asbp_fbhealth) (/ (Variables|Default|GetHealth_FB) 1e+02))
  (Transformation|SetWorldRotation _health_bar_widget (Math|Rotator|FindLookatRotation (Transformation|GetWorldLocation _health_bar_widget) (Transformation|GetWorldLocation (Variables|/Script/Engine.PlayerCameraManager|GetTransformComponent (Game|GetPlayerCameraManager 0)))) false false))

(fn ConstructionScript)