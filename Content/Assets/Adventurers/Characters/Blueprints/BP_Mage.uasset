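; Mage Blueprint that spawns three BP_MageRoam actors at the world transforms of its three arrow components.
; BeginPlay and PawnSensing's OnSeePawn share that spawn chain, which also switches off sensing updates.
; Because BeginPlay runs the chain, spawning and sensing shutdown happen at start without waiting for a sighting.
; A looping two-handed melee idle animation node is left unconnected.
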(event OnSeePawn(PawnSensing)
  (params (Pawn :type Pawn%20Object%20Reference))
  (for _array_element (Utilities|Array|MakeArray (Variables|Default|GetArrow1) (Variables|Default|GetArrow2) (Variables|Default|GetArrow3))
    (Game|SpawnActorfromClass "/Game/Assets/Adventurers/Characters/Blueprints/BP_MageRoam.BP_MageRoam_C" (Transformation|GetWorldTransform _array_element) "Undefined" 0 0)
    (Class|PawnSensingComponent|SetSensingUpdatesEnabled (Variables|Default|GetPawnSensing) false)))

(event EventBeginPlay
  (for _array_element (Utilities|Array|MakeArray (Variables|Default|GetArrow1) (Variables|Default|GetArrow2) (Variables|Default|GetArrow3))
    (Game|SpawnActorfromClass "/Game/Assets/Adventurers/Characters/Blueprints/BP_MageRoam.BP_MageRoam_C" (Transformation|GetWorldTransform _array_element) "Undefined" 0 0)
    (Class|PawnSensingComponent|SetSensingUpdatesEnabled (Variables|Default|GetPawnSensing) false)))

(fn ConstructionScript)