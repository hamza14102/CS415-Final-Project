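; Final boss enemy that roams, chases pawns it sees and can fire arrows.
; BeginPlay plays a walk animation and starts one move to a random reachable point nearby.
; PawnSensing sightings switch to running, interpolate yaw toward the pawn with a debug print, then move to its location after a short delay.
; KeepShooting re-calls itself after a delay to spawn BP_Arrow from Arrow1, but nothing here starts it.
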(event OnSeePawn(PawnSensing)
  (params (Pawn :type Pawn%20Object%20Reference))
  (bind _returnvalue (Utilities|Time|GetWorldDeltaSeconds))
  (bind _returnvalue_2 (Transformation|GetActorLocation Pawn))
  (bind _self self)
  (bind _returnvalue_3 (Transformation|GetActorLocation _self))
  (bind _returnvalue_4 (Transformation|GetActorRotation _self))
  (bind _returnvalue_5 (Math|Rotator|FindLookatRotation _returnvalue_3 _returnvalue_2))
  (bind _returnvalue_6 (Math|Interpolation|RInterpTo _returnvalue_4 _returnvalue_5 _returnvalue 2e+01))
  (Components|Animation|PlayAnimation (Variables|Character|GetMesh) "/Game/Assets/Adventurers/Characters/Rogue/Rogue_Anim_Running_A.Rogue_Anim_Running_A" true)
  (Transformation|SetActorRotation _self (Math|Rotator|MakeRotator 0.0 0.0 (.yaw _returnvalue_6)))
  (Development|PrintString (Utilities|String|ToString(Float) (.yaw _returnvalue_6)))
  (Utilities|FlowControl|Delay 0.2)
  (AI|AIMoveTo _self _returnvalue_2 0 5.0 false
    (:then
      (Utilities|FlowControl|Delay 0.3))))

(event Custom|KeepShooting
  (bind _arrow1 (Variables|Default|GetArrow1))
  (bind _returnvalue (Transformation|GetWorldTransform _arrow1))
  (Game|SpawnActorfromClass "/Game/FinalLevel/FinalBoss/BP_Arrow.BP_Arrow_C" (Math|Transform|MakeTransform (.location _returnvalue) (Math|Rotator|MakeRotator (.roll (.rotation _returnvalue)) 0.0 0.0) (.scale _returnvalue)) "Undefined" 0 0)
  (Utilities|FlowControl|Delay 1.0)
  (CallFunction|KeepShooting))

(event Custom|Roam
  (AI|AIMoveTo self (.RandomLocation (AI|Navigation|GetRandomReachablePointinRadius (Transformation|GetActorLocation) 2e+03 0 0)) 0 5.0 false))

(event EventBeginPlay
  (Components|Animation|PlayAnimation (Variables|Character|GetMesh) "/Game/Assets/Adventurers/Characters/Rogue/Rogue_Anim_Walking_A.Rogue_Anim_Walking_A" true)
  (CallFunction|Roam))

(fn ConstructionScript)